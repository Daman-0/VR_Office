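; AI controller for Slenderman that runs the SlendermanBehaviour tree and feeds it what the character sees and hears.
; Each perception update goes to sight and hearing handlers, which filter by sense class and write to the Blackboard.
; Sight sets TargetActor while the player is seen, then clears it and stores LastKnowLocation when sight is lost.
; Hearing writes any stimulus location to TargetLocation, without checking its source.
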(event `self.ReceiveBeginPlay`
  (`self.RunBehaviorTree` "/Game/Characters/SlenderMan/Blueprint/SlendermanBehaviour.SlendermanBehaviour"))

(event `self.AIPerception.OnTargetPerceptionUpdated`
  (params (Actor :type "Actor Object Reference") (Stimulus :type "AIStimulus Structure"))
  (`self.Handle Sight Sense` Actor Stimulus)
  (`self.Handle Hearing Sense` Stimulus))

(fn `Handle Hearing Sense`
  (params (Stimulus :type "AIStimulus Structure (by ref)"))
  (bind _returnvalue (`AIPerceptionSystem.GetSenseClassForStimulus` Stimulus))
  (if (== _returnvalue "/Script/AIModule.AISense_Hearing")
    (`BlackboardComponent.SetValueAsVector` (`self.Blackboard`) "TargetLocation" (`.StimulusLocation` (break `AIStimulus` Stimulus)))))

(fn `Handle Sight Sense`
  (params (Actor :type "Actor Object Reference") (Stimulus :type "AIStimulus Structure"))
  (locals (NewLocalVar :type "Actor Object Reference"))
  (bind (_age _expirationage _strength _stimuluslocation _receiverlocation _tag _bsuccessfullysensed) (break `AIStimulus` (`local.Stimulus`)))
  (bind _returnvalue (`AIPerceptionSystem.GetSenseClassForStimulus` Stimulus))
  (if (== _returnvalue "/Script/AIModule.AISense_Sight")
    (if (== Actor (`GameplayStatics.GetPlayerCharacter` 0))
      (`BlackboardComponent.SetValueAsObject` (`self.Blackboard`) "TargetActor" (`KismetMathLibrary.SelectObject` (`GameplayStatics.GetPlayerCharacter` 0) null _bsuccessfullysensed))
      (if (not _bsuccessfullysensed)
        (`BlackboardComponent.SetValueAsVector` (`self.Blackboard`) "LastKnowLocation" _stimuluslocation))
      (else
        (return)))
    (else
      (return))))

(fn `UserConstructionScript`)