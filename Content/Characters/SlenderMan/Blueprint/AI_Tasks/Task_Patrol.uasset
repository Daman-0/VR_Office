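; Behavior tree task that makes the controlled pawn, under the SlenderMan character assets, patrol a looping route.
; It reads the PatrolPath map from the pawn's AI_Behaviour component, using keys as destination actors and values as wait times.
; Each successful AI MoveTo starts a timer that advances the index, wrapping at the end.
; The task never finishes successfully, only failing on a missing component, empty path or failed move.
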(event `self.ReceiveExecuteAI`
  (params (OwnerController :type "AIController Object Reference") (ControlledPawn :type "Pawn Object Reference"))
  (bind _returnvalue (`Actor.GetComponentByClass` ControlledPawn "/Game/VRTemplate/Blueprints/AI_Behaviour.AI_Behaviour_C"))
  (bind _patrolpath (`/Game/VRTemplate/Blueprints/AI_Behaviour.PatrolPath` _returnvalue))
  (set `self.Controlled Pawn` ControlledPawn)
  (`/Engine/EditorBlueprintResources/StandardMacros.IsValid` _returnvalue
    (:`Is Valid`
      (if (> (`BlueprintMapLibrary.Map_Length` _patrolpath) 0)
        (set `self.Patrol Path` _patrolpath)
        (`self.MovePatrol`)
        (else
          (`self.FinishExecute` false))))
    (:`Is Not Valid`
      (`self.FinishExecute` false))))

(event `MovePatrol`
  (bind _patrol_path (`self.Patrol Path`))
  (bind _keys (`BlueprintMapLibrary.Map_Keys` (`self.Patrol Path`)))
  (`|AIMoveTo` (`self.Controlled Pawn`) (`Actor.K2_GetActorLocation` (`|GetArrayItem` _keys (`self.CurrentIndex`))) null
    (:`OnSuccess`
      (bind _keys_2 (`BlueprintMapLibrary.Map_Keys` _patrol_path))
      (`KismetSystemLibrary.K2_SetTimerDelegate` (delegate `WaitTime`) (`KismetMathLibrary.FMax` (`BlueprintMapLibrary.Map_Find` _patrol_path (`|GetArrayItem` _keys_2 (`self.CurrentIndex`))) 0.1)))
    (:`OnFail`
      (`self.FinishExecute` false))))

(event `WaitTime`
  (bind _result (`/Engine/EditorBlueprintResources/StandardMacros.IncrementInt` (`self.CurrentIndex`))
    (:`  `
      (if (>= _result (`BlueprintMapLibrary.Map_Length` (`self.Patrol Path`)))
        (set `self.CurrentIndex` 0)
        (`self.MovePatrol`)
        (else
          (`self.MovePatrol`))))))